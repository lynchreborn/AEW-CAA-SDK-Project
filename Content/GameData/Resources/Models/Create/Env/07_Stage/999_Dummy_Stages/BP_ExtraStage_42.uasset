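; Custom wrestling stage actor that strips selected default arena pieces (ring, lights, LED panels, barricades, audience) and can reskin the crowd.
; Tick feeds a one-second Delay into DestroyAllFunctions, repeatedly running bool-gated GetAllActorsOfClass sweeps.
; These sweeps destroy matching actors, except stage floor and ramp pieces, which are hidden with collision disabled.
; 1.5 seconds after BeginPlay, SetCrowdMaterial optionally gives each BP_Audience one of seven random materials.
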(event EventBeginPlay
  (|CallParentFunction)
  (Utilities|FlowControl|Delay 1.5)
  (CallFunction|SetCrowdMaterial))

(event Collision|EventActorBeginOverlap
  (params (OtherActor :type Actor%20Object%20Reference))
  (|CallParentFunction OtherActor) ; This node is disabled and will not be called.\nDrag off pins to build functionality.
)

(event EventTick
  (params (DeltaSeconds :type Float%20%28single-precision%29))
  (|CallParentFunction DeltaSeconds)
  (Utilities|FlowControl|Delay 1.0)
  (Utilities|DestroyAllFunctions))

(fn ConstructionScript
  (|CallParentFunction))

(fn DestroyRing
  (if (Variables|Ring|GetEntireRing)
    (bind _outactors (Actor|GetAllActorsOfClass "/Game/GameData/Assets/Ring/BP_Ring.BP_Ring_C"))
    (for _array_element _outactors
      (Actor|DestroyActor _array_element))))

(fn DestroyCurtain01
  (if (Variables|Stage|GetCurtain01)
    (bind _outactors (Actor|GetAllActorsOfClass "/Game/GameData/Resources/Models/EmvData/01_AEW_Dynamite/0008_Stage/BP_Stage_Curtain01.BP_Stage_Curtain01_C"))
    (for _array_element _outactors
      (Actor|DestroyActor _array_element))))

(fn DestroySteelSteps
  (if (Variables|Ring|GetSteelSteps)
    (bind _outactors (Actor|GetAllActorsOfClass "/Game/GameData/Assets/Ring/BP_SteelStep.BP_SteelStep_C"))
    (for _array_element _outactors
      (Actor|DestroyActor _array_element))))

(fn DestroyASFFirstFloor
  (if (Variables|Stadium|GetASFFirstFloor)
    (bind _outactors (Actor|GetAllActorsOfClass "/Game/GameData/Resources/Models/EmvData/0000_01_Atlanta_State_Farm/BP_ASF_Parts01_FirstFloor_Grp.BP_ASF_Parts01_FirstFloor_Grp_C"))
    (for _array_element _outactors
      (Actor|DestroyActor _array_element))))

(fn DestroyCorridorLights
  (if (Variables|Stadium|GetASFCorridorLights)
    (bind _outactors (Actor|GetAllActorsOfClass "/Game/GameData/Resources/Models/EmvData/0000_01_Atlanta_State_Farm/BP_CorridorLights.BP_CorridorLights_C"))
    (for _array_element _outactors
      (Actor|DestroyActor _array_element))))

(fn DestroyHandrail01
  (if (Variables|Stadium|GetASFHandrail01)
    (bind _outactors (Actor|GetAllActorsOfClass "/Game/GameData/Resources/Models/EmvData/0000_01_Atlanta_State_Farm/BP_Handrail01.BP_Handrail01_C"))
    (for _array_element _outactors
      (Actor|DestroyActor _array_element))))

(fn DestroyOtherMeshes
  (if (Variables|Stadium|GetASFOtherStaticMeshes)
    (bind _outactors (Actor|GetAllActorsOfClass "/Game/GameData/Resources/Models/EmvData/0000_01_Atlanta_State_Farm/BP_Other_StaticMeshes.BP_Other_StaticMeshes_C"))
    (for _array_element _outactors
      (Actor|DestroyActor _array_element))))

(fn DestroyLEDPanel1
  (if (Variables|Stadium|GetAEWLEDPanel1)
    (bind _outactors (Actor|GetAllActorsOfClass "/Game/GameData/Resources/Models/EmvData/01_AEW_Dynamite/0012_Panel/BP_Panel_01.BP_Panel_01_C"))
    (for _array_element _outactors
      (Actor|DestroyActor _array_element))))

(fn DestroyLEDPanel2
  (if (Variables|Stadium|GetAEWLEDPanel01set)
    (bind _outactors (Actor|GetAllActorsOfClass "/Game/GameData/Resources/Models/EmvData/01_AEW_Dynamite/0012_Panel/BP_Panel_01Set.BP_Panel_01Set_C"))
    (for _array_element _outactors
      (Actor|DestroyActor _array_element))))

(fn DestroyLEDPanel3
  (if (Variables|Stadium|GetAEWLEDPanel01set)
    (bind _outactors (Actor|GetAllActorsOfClass "/Game/GameData/Resources/Models/EmvData/01_AEW_Dynamite/0012_Panel/BP_Panel_02.BP_Panel_02_C"))
    (for _array_element _outactors
      (Actor|DestroyActor _array_element))))

(fn DestroyLEDPanel4
  (if (Variables|Stadium|GetAEWLEDPanel3)
    (bind _outactors (Actor|GetAllActorsOfClass "/Game/GameData/Resources/Models/EmvData/01_AEW_Dynamite/0012_Panel/BP_Panel_03.BP_Panel_03_C"))
    (for _array_element _outactors
      (Actor|DestroyActor _array_element))))

(fn DestroyAisleLight
  (if (Variables|Light|GetAisleLight1)
    (bind _outactors (Actor|GetAllActorsOfClass "/Game/GameData/Resources/Models/EmvData/01_AEW_Dynamite/0009_AisleLight/BP_Aisle_Light_01.BP_Aisle_Light_01_C"))
    (for _array_element _outactors
      (Actor|DestroyActor _array_element))))

(fn DestroyAisleLightgp
  (if (Variables|Light|GetAisleLightGP)
    (bind _outactors (Actor|GetAllActorsOfClass "/Game/GameData/Resources/Models/EmvData/01_AEW_Dynamite/0009_AisleLight/BP_Aisle_Light_Gp.BP_Aisle_Light_Gp_C"))
    (for _array_element _outactors
      (Actor|DestroyActor _array_element))))

(fn DestroyRingAprons
  (if (Variables|Ring|GetRing_Aprons)
    (bind _outactors (Actor|GetAllActorsOfClass "/Game/GameData/Resources/Models/EmvData/Arean/Common/Apron/0001_Dynamite/BP_Apron_0001.BP_Apron_0001_C"))
    (for _array_element _outactors
      (Actor|DestroyActor _array_element))))

(fn DestroyCornerJoints
  (if (Variables|Ring|GetRing_CornerJoint)
    (bind _outactors (Actor|GetAllActorsOfClass "/Game/GameData/Resources/Models/EmvData/Arean/Common/CornerJoint/0000_Base/BP_CornerJoint.BP_CornerJoint_C"))
    (for _array_element _outactors
      (Actor|DestroyActor _array_element))))

(fn DestroyCornerPosts
  (if (Variables|Ring|GetCorner%20Posts)
    (bind _outactors (Actor|GetAllActorsOfClass "/Game/GameData/Resources/Models/EmvData/Arean/Common/CornerPost/0000_Base/BP_Cornerpost.BP_Cornerpost_C"))
    (for _array_element _outactors
      (Actor|DestroyActor _array_element))))

(fn DestroyRampLED01
  (if (Variables|Light|GetRamp_LED01)
    (bind _outactors (Actor|GetAllActorsOfClass "/Game/GameData/Resources/Models/EmvData/Arean/Common/WallWasherLight/0001_Dynamite/BP_Ramp_LED_Rect_01.BP_Ramp_LED_Rect_01_C"))
    (for _array_element _outactors
      (Actor|DestroyActor _array_element))))

(fn DestroyRampLED02
  (if (Variables|Light|GetRamp_LED02)
    (bind _outactors (Actor|GetAllActorsOfClass "/Game/GameData/Resources/Models/EmvData/Arean/Common/WallWasherLight/0001_Dynamite/BP_Ramp_LED_Rect_02.BP_Ramp_LED_Rect_02_C"))
    (for _array_element _outactors
      (Actor|DestroyActor _array_element))))

(fn DestroyRingMat
  (if (Variables|Ring|GetRingMat)
    (bind _outactors (Actor|GetAllActorsOfClass "/Game/GameData/Resources/Models/EmvData/Arean/Common/RingMat/0000_Base/BP_RingMat.BP_RingMat_C"))
    (for _array_element _outactors
      (Actor|DestroyActor _array_element))))

(fn DestroyRopes
  (if (Variables|Ring|GetRopes)
    (bind _outactors (Actor|GetAllActorsOfClass "/Game/GameData/Assets/Ring/BP_Ropes.BP_Ropes_C"))
    (for _array_element _outactors
      (Actor|DestroyActor _array_element))))

(fn DestroyTurnbuckleCover
  (if (Variables|Ring|GetTurnbuckle%20Cover)
    (bind _outactors (Actor|GetAllActorsOfClass "/Game/GameData/Resources/Models/EmvData/Arean/Common/TB_Cover/0000_Base/BP_TB_Cover.BP_TB_Cover_C"))
    (for _array_element _outactors
      (Actor|DestroyActor _array_element))))

(fn DestroyStructLight01
  (if (Variables|Stadium|GetStructLight01)
    (bind _outactors (Actor|GetAllActorsOfClass "/Game/GameData/Resources/Models/EmvData/01_AEW_Dynamite/0011_StructureLight/BP_Structure_Light_01.BP_Structure_Light_01_C"))
    (for _array_element _outactors
      (Actor|DestroyActor _array_element))))

(fn DestroyStructLight02
  (if (Variables|Stadium|GetStructLight02)
    (bind _outactors (Actor|GetAllActorsOfClass "/Game/GameData/Resources/Models/EmvData/01_AEW_Dynamite/0011_StructureLight/BP_Structure_Light_02.BP_Structure_Light_02_C"))
    (for _array_element _outactors
      (Actor|DestroyActor _array_element))))

(fn DestroyStructLight05
  (if (Variables|Stadium|GetStructLight05)
    (bind _outactors (Actor|GetAllActorsOfClass "/Game/GameData/Resources/Models/EmvData/01_AEW_Dynamite/0011_StructureLight/BP_Structure_light05.BP_Structure_light05_C"))
    (for _array_element _outactors
      (Actor|DestroyActor _array_element))))

(fn DestroyASFUniqueGrp
  (if (Variables|Stadium|GetASFUniqueSecGroup)
    (bind _outactors (Actor|GetAllActorsOfClass "/Game/GameData/Resources/Models/EmvData/0000_01_Atlanta_State_Farm/BP_Uniqe_SectionGrp.BP_Uniqe_SectionGrp_C"))
    (for _array_element _outactors
      (Actor|DestroyActor _array_element))))

(fn DestroyBarricade
  (if (Variables|Ring|GetBarricade)
    (bind _outactors (Actor|GetAllActorsOfClass "/Game/GameData/Resources/Models/EmvData/Arean/Common/Barricade/0001_Dynamite/BP_Barricade_0001.BP_Barricade_0001_C"))
    (for _array_element _outactors
      (Actor|DestroyActor _array_element))))

(fn DestroyBarricadeLong
  (if (Variables|Ring|GetBarricade_Long)
    (bind _outactors (Actor|GetAllActorsOfClass "/Game/GameData/Resources/Models/EmvData/Arean/Common/Barricade/0001_Dynamite/BP_Barricade_Long_0001.BP_Barricade_Long_0001_C"))
    (for _array_element _outactors
      (Actor|DestroyActor _array_element))))

(fn DestroyFloorGroup
  (if (Variables|Stage|GetFloor01_Group)
    (bind _outactors (Actor|GetAllActorsOfClass "/Game/GameData/Resources/Models/EmvData/01_AEW_Dynamite/0008_Stage/BP_Floor01_Grp.BP_Floor01_Grp_C"))
    (for _array_element _outactors
      (Actor|DestroyActor _array_element))))

(fn DestroyStageLightOthers
  (if (Variables|Light|GetStageLight_Others)
    (bind _outactors (Actor|GetAllActorsOfClass "/Game/GameData/Resources/Models/EmvData/01_AEW_Dynamite/0006_StageLight/Stage_Others_01.Stage_Others_01_C"))
    (for _array_element _outactors
      (Actor|DestroyActor _array_element))))

(fn DestroyStageLight01
  (if (Variables|Light|GetStageLight01)
    (bind _outactors (Actor|GetAllActorsOfClass "/Game/GameData/Resources/Models/EmvData/Arean/Common/StageLight/0000_Base/BP_StageLight1.BP_StageLight1_C"))
    (for _array_element _outactors
      (Actor|DestroyActor _array_element))))

(fn DestroyStageLightOthers2
  (if (Variables|Light|GetStageLight_Others2)
    (bind _outactors (Actor|GetAllActorsOfClass "/Game/GameData/Resources/Models/EmvData/01_AEW_Dynamite/0006_StageLight/Stage_Others_02.Stage_Others_02_C"))
    (for _array_element _outactors
      (Actor|DestroyActor _array_element))))

(fn DestroyStageLightOthers3
  (if (Variables|Light|GetStageLight_Others3)
    (bind _outactors (Actor|GetAllActorsOfClass "/Game/GameData/Resources/Models/EmvData/01_AEW_Dynamite/0006_StageLight/Stage_Others_03.Stage_Others_03_C"))
    (for _array_element _outactors
      (Actor|DestroyActor _array_element))))

(fn DestroyStageLightOthers4
  (if (Variables|Light|GetStageLight_Others4)
    (bind _outactors (Actor|GetAllActorsOfClass "/Game/GameData/Resources/Models/EmvData/01_AEW_Dynamite/0006_StageLight/Stage_Others_04.Stage_Others_04_C"))
    (for _array_element _outactors
      (Actor|DestroyActor _array_element))))

(fn DestroyAudience
  (if (Variables|Ring|GetAudience)
    (bind _outactors (Actor|GetAllActorsOfClass "/Game/GameData/Assets/Audience/BP_Audience.BP_Audience_C"))
    (for _array_element _outactors
      (Actor|DestroyActor _array_element))))

(fn DestroyWallWasherLight
  (if (Variables|Light|GetWallWasherLight)
    (bind _outactors (Actor|GetAllActorsOfClass "/Game/GameData/Resources/Models/EmvData/Arean/Common/WallWasherLight/0000_Base/BP_WallWasherLight.BP_WallWasherLight_C"))
    (for _array_element _outactors
      (Actor|DestroyActor _array_element))))

(fn DestroyStageFloor
  (if (Variables|Stage|GetStage_Floor)
    (bind _outactors (Actor|GetAllActorsOfClass "/Game/GameData/Resources/Models/EmvData/01_AEW_Dynamite/0008_Stage/BP_Stage_Floor01.BP_Stage_Floor01_C"))
    (for _array_element _outactors
      (Rendering|SetActorHiddenInGame _array_element true)
      (Collision|SetActorEnableCollision _array_element false))))

(fn DestroyGroundMat
  (if (Variables|Ring|GetGround%20Mat)
    (bind _outactors (Actor|GetAllActorsOfClass "/Game/GameData/Resources/Models/EmvData/Arean/Common/GroundMat/0000_Base/BP_GroundMat_Base.BP_GroundMat_Base_C"))
    (for _array_element _outactors
      (Actor|DestroyActor _array_element))))

(fn DestroyTBCoverNJPW
  (if (Variables|Ring|GetTB_Cover_NJPW)
    (bind _outactors (Actor|GetAllActorsOfClass "/Game/GameData/Resources/Models/EmvData/Arean/Common/TB_Cover/0000_Base/BP_TB_Cover_Type02.BP_TB_Cover_Type02_C"))
    (for _array_element _outactors
      (Actor|DestroyActor _array_element))))

(fn DestroyRampLights
  (if (Variables|Light|GetRamp_OtherLights)
    (bind _outactors (Actor|GetAllActorsOfClass "/Game/GameData/Resources/Models/EmvData/Arean/Common/Other_Light/BP_StageRampOtherLight.BP_StageRampOtherLight_C"))
    (for _array_element _outactors
      (Actor|DestroyActor _array_element))))

(fn DestroyRampLightsColor01
  (if (Variables|Light|GetRamp_SLights_Color_01)
    (bind _outactors (Actor|GetAllActorsOfClass "/Game/GameData/Resources/Models/EmvData/01_AEW_Dynamite/0006_StageLight/BP_Ramp_SL_Color_01Set.BP_Ramp_SL_Color_01Set_C"))
    (for _array_element _outactors
      (Actor|DestroyActor _array_element))))

(fn DestroyRampLEDCol02
  (if (Variables|Light|GetRamp_LED_Col02)
    (bind _outactors (Actor|GetAllActorsOfClass "/Game/GameData/Resources/Models/EmvData/Arean/Common/WallWasherLight/0001_Dynamite/BP_Ramp_LED_Color_02.BP_Ramp_LED_Color_02_C"))
    (for _array_element _outactors
      (Actor|DestroyActor _array_element))))

(fn DestroyRampLEDCol01
  (if (Variables|Light|GetRamp_LED_Col01)
    (bind _outactors (Actor|GetAllActorsOfClass "/Game/GameData/Resources/Models/EmvData/Arean/Common/WallWasherLight/0001_Dynamite/BP_Ramp_LED_Color_01.BP_Ramp_LED_Color_01_C"))
    (for _array_element _outactors
      (Actor|DestroyActor _array_element))))

(fn DestroyRamp
  (if (Variables|Stage|GetRamp_Floor)
    (bind _outactors (Actor|GetAllActorsOfClass "/Game/GameData/Resources/Models/EmvData/Arean/Common/Ramp/BP_Ramp.BP_Ramp_C"))
    (for _array_element _outactors
      (Rendering|SetActorHiddenInGame _array_element true)
      (Collision|SetActorEnableCollision _array_element false))))

(fn DestroyRampFloor
  (if (Variables|Stage|GetRamp_Floor)
    (bind _outactors (Actor|GetAllActorsOfClass "/Game/GameData/Resources/Models/EmvData/01_AEW_Dynamite/0008_Stage/BP_Ramp_Floor01.BP_Ramp_Floor01_C"))
    (for _array_element _outactors
      (Rendering|SetActorHiddenInGame _array_element true)
      (Collision|SetActorEnableCollision _array_element false))))

(fn DestroyLightGrp1
  (if (Variables|Light|GetLight_Grp_1)
    (bind _outactors (Actor|GetAllActorsOfClass "/Game/GameData/Resources/Models/EmvData/01_AEW_Dynamite/0011_StructureLight/BP_SF_01_Grp.BP_SF_01_Grp_C"))
    (for _array_element _outactors
      (Actor|DestroyActor _array_element))))

(fn DestroyLightGrp2
  (if (Variables|Light|GetLight_Grp_2)
    (bind _outactors (Actor|GetAllActorsOfClass "/Game/GameData/Resources/Models/EmvData/01_AEW_Dynamite/0011_StructureLight/BP_SF_02_Grp.BP_SF_02_Grp_C"))
    (for _array_element _outactors
      (Actor|DestroyActor _array_element))))

(fn DestroyLightGrp3
  (if (Variables|Light|GetLight_Grp3)
    (bind _outactors (Actor|GetAllActorsOfClass "/Game/GameData/Resources/Models/EmvData/01_AEW_Dynamite/0011_StructureLight/BP_SF_03_Grp.BP_SF_03_Grp_C"))
    (for _array_element _outactors
      (Actor|DestroyActor _array_element))))

(fn DestroyLightSL3
  (if (Variables|Light|GetLightSL_Grp_3)
    (bind _outactors (Actor|GetAllActorsOfClass "/Game/GameData/Resources/Models/EmvData/01_AEW_Dynamite/0011_StructureLight/BP_SL_03_Grp.BP_SL_03_Grp_C"))
    (for _array_element _outactors
      (Actor|DestroyActor _array_element))))

(fn DestroySLBlue01
  (if (Variables|Light|GetSL_Blue01)
    (bind _outactors (Actor|GetAllActorsOfClass "/Game/GameData/Resources/Models/EmvData/01_AEW_Dynamite/0011_StructureLight/BP_SL_Blue_01_Grp.BP_SL_Blue_01_Grp_C"))
    (for _array_element _outactors
      (Actor|DestroyActor _array_element))))

(fn DestroySLBlue02
  (if (Variables|Light|GetSL_Blue02)
    (bind _outactors (Actor|GetAllActorsOfClass "/Game/GameData/Resources/Models/EmvData/01_AEW_Dynamite/0011_StructureLight/BP_SL_Blue_02_Grp.BP_SL_Blue_02_Grp_C"))
    (for _array_element _outactors
      (Actor|DestroyActor _array_element))))

(fn DestroySLRed02
  (if (Variables|Light|GetSL_Red02)
    (bind _outactors (Actor|GetAllActorsOfClass "/Game/GameData/Resources/Models/EmvData/01_AEW_Dynamite/0011_StructureLight/BP_SL_Red_02_Grp.BP_SL_Red_02_Grp_C"))
    (for _array_element _outactors
      (Actor|DestroyActor _array_element))))

(fn DestroyLEDBlue
  (if (Variables|Light|GetLED_Blue_02)
    (bind _outactors (Actor|GetAllActorsOfClass "/Game/GameData/Resources/Models/EmvData/01_AEW_Dynamite/0011_StructureLight/BP_LED_Blue_02_GRP.BP_LED_Blue_02_GRP_C"))
    (for _array_element _outactors
      (Actor|DestroyActor _array_element))))

(fn DestroyStructLight06
  (if (Variables|Light|GetStructLight06)
    (bind _outactors (Actor|GetAllActorsOfClass "/Game/GameData/Resources/Models/EmvData/01_AEW_Dynamite/0011_StructureLight/BP_Structure_light06.BP_Structure_light06_C"))
    (for _array_element _outactors
      (Actor|DestroyActor _array_element))))

(fn DestroyLEDRed02
  (if (Variables|Light|GetLED_Red_02)
    (bind _outactors (Actor|GetAllActorsOfClass "/Game/GameData/Resources/Models/EmvData/01_AEW_Dynamite/0011_StructureLight/BP_LED_Red_02_GRP.BP_LED_Red_02_GRP_C"))
    (for _array_element _outactors
      (Actor|DestroyActor _array_element))))

(fn DestroyLEDBlue03
  (if (Variables|Light|GetLED_Blue_03)
    (bind _outactors (Actor|GetAllActorsOfClass "/Game/GameData/Resources/Models/EmvData/01_AEW_Dynamite/0011_StructureLight/BP_LED_Blue_03_Grp2.BP_LED_Blue_03_Grp2_C"))
    (for _array_element _outactors
      (Actor|DestroyActor _array_element))))

(fn DestroyLEDRed03
  (if (Variables|Light|GetLED_Red_03)
    (bind _outactors (Actor|GetAllActorsOfClass "/Game/GameData/Resources/Models/EmvData/01_AEW_Dynamite/0011_StructureLight/BP_LED_Red_03_Grp2.BP_LED_Red_03_Grp2_C"))
    (for _array_element _outactors
      (Actor|DestroyActor _array_element))))

(fn DestroyDynStageLED01
  (if (Variables|Light|GetDyn_Stage_LED_01)
    (bind _outactors (Actor|GetAllActorsOfClass "/Game/GameData/Resources/Models/EmvData/01_AEW_Dynamite/0007_WallWasherLight/BP_Stage_LED_Color_01.BP_Stage_LED_Color_01_C"))
    (for _array_element _outactors
      (Actor|DestroyActor _array_element))))

(fn DestroyDynStageLED010
  (if (Variables|Light|GetDyn_Stage_LED_02)
    (bind _outactors (Actor|GetAllActorsOfClass "/Game/GameData/Resources/Models/EmvData/01_AEW_Dynamite/0007_WallWasherLight/BP_Stage_LED_Color_02.BP_Stage_LED_Color_02_C"))
    (for _array_element _outactors
      (Actor|DestroyActor _array_element))))

(fn SetRandomAud
  (params (Aud1 :type Material%20Instance%20Object%20Reference) (Aud2 :type Material%20Instance%20Object%20Reference) (Aud3 :type Material%20Instance%20Object%20Reference) (Aud4 :type Material%20Instance%20Object%20Reference) (Aud5 :type Material%20Instance%20Object%20Reference) (Aud6 :type Material%20Instance%20Object%20Reference) (Aud7 :type Material%20Instance%20Object%20Reference))
  (switch int (Math|Random|RandomIntegerinRange 0 6)
    (:Default
      _)
    (:0
      (return Aud1))
    (:1
      (return Aud2))
    (:2
      (return Aud3))
    (:3
      _)
    (:4
      (return Aud5))
    (:5
      (return Aud6))
    (:6
      (return Aud7)))
  (return Aud4))

(fn SetCrowdMaterial
  (if (Variables|Ring|GetUseCustomAudience?)
    (bind _outactors (Actor|GetAllActorsOfClass "/Game/GameData/Assets/Audience/BP_Audience.BP_Audience_C"))
    (for _array_element _outactors
      (bind _output_aud (CallFunction|SetRandomAud (Variables|Aud|GetAud1) (Variables|Aud|GetAud2) (Variables|Aud|GetAud3) (Variables|Aud|GetAud4) (Variables|Aud|GetAud5) (Variables|Aud|GetAud6) (Variables|Aud|GetAud7)))
      (Rendering|Material|SetMaterial (Actor|GetComponentbyClass _array_element "/Script/Engine.SkeletalMeshComponent") 0 _output_aud))))

(fn DestroyBPStageSL01
  (if (Variables|Light|GetBP_Stage_SL_01)
    (bind _outactors (Actor|GetAllActorsOfClass "/Game/GameData/Resources/Models/EmvData/01_AEW_Dynamite/0006_StageLight/BP_Stage_SL_01.BP_Stage_SL_01_C"))
    (for _array_element _outactors
      (Actor|DestroyActor _array_element))))

(fn DestroyBPStageLEDColor0105
  (if (Variables|Light|GetBP_Stage_LED_Color_01_05)
    (bind _outactors (Actor|GetAllActorsOfClass "/Game/GameData/Resources/Models/EmvData/05_Revolution/BP_Stage_LED_Color_01_05.BP_Stage_LED_Color_01_05_C"))
    (for _array_element _outactors
      (Actor|DestroyActor _array_element))))

(fn DestroyBPStageSL02
  (if (Variables|Light|GetBP_Stage_SL_02)
    (bind _outactors (Actor|GetAllActorsOfClass "/Game/GameData/Resources/Models/EmvData/01_AEW_Dynamite/0006_StageLight/BP_Stage_SL_02.BP_Stage_SL_02_C"))
    (for _array_element _outactors
      (Actor|DestroyActor _array_element))))

(fn DestroyBPStageLEDColor0205
  (if (Variables|Light|GetBP_Stage_LED_Color_02_05)
    (bind _outactors (Actor|GetAllActorsOfClass "/Game/GameData/Resources/Models/EmvData/05_Revolution/BP_Stage_LED_Color_02_05.BP_Stage_LED_Color_02_05_C"))
    (for _array_element _outactors
      (Actor|DestroyActor _array_element))))

(fn DestroyBPRampLEDColor0105
  (if (Variables|Light|GetBP_Ramp_LED_Color_01_05)
    (bind _outactors (Actor|GetAllActorsOfClass "/Game/GameData/Resources/Models/EmvData/05_Revolution/BP_Ramp_LED_Color_01_05.BP_Ramp_LED_Color_01_05_C"))
    (for _array_element _outactors
      (Actor|DestroyActor _array_element))))

(fn DestroyBPRampLEDColor0205
  (if (Variables|Light|GetBP_Ramp_LED_Color_02_05)
    (bind _outactors (Actor|GetAllActorsOfClass "/Game/GameData/Resources/Models/EmvData/05_Revolution/BP_Ramp_LED_Color_02_05.BP_Ramp_LED_Color_02_05_C"))
    (for _array_element _outactors
      (Actor|DestroyActor _array_element))))